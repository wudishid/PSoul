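; Base AI controller Blueprint that runs an assigned behavior tree on BeginPlay and feeds it a target from AI perception.
; When perception updates, a helper function measures the controlled pawn's distance to each updated actor and returns the closest one.
; A valid result is written to the Blackboard "Target" key, which this Blueprint never clears.
; The helper selects purely by distance, with no team, class or sensing-state check.
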(event OnPerceptionUpdated(AIPerception)
  (params (UpdatedActors :type Array%20of%20Actor%20Object%20References))
  (bind _target (CallFunction|FFilterActorsasTarget UpdatedActors))
  (Utilities|IsValid _target
    (:Is%20Valid
      (AI|Components|Blackboard|SetValueasObject (AI|GetBlackboard 0) (Utilities|Name|MakeLiteralName "Target") _target))))

(event EventBeginPlay
  (AI|RunBehaviorTree (Variables|Default|GetBTAsset)))

(event EventTick
  (params (DeltaSeconds :type Float%20%28single-precision%29)))

(fn ConstructionScript)

(fn FFilterActorsasTarget
  (params (Actors :type Array%20of%20Actor%20Object%20References))
  (for _array_element Actors
    (Utilities|Array|Add (LocalVariables|GetTemp_Distances) (Transformation|GetDistanceTo (Pawn|GetControlledPawn) _array_element)))
  (return (Utilities|Array|Get(acopy) Actors (.IndexOfMinValue (Math|Float|MinOfFloatArray (LocalVariables|GetTemp_Distances))))))