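; GA_Death_Player is a Gameplay Ability that runs the player's death sequence.
; On activation it plays one of two death montages at random, ANMTG_Death_F or ANMTG_Death_B.
; It ignores the montage callbacks and waits on a Delay sized by the separate DeathMontage variable, not the montage chosen.
; It then calls FinishDeath on the owning PlayerCharacterBase and ends the ability.
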(event Ability|EventOnEndAbility
  (params (bWasCancelled :type Boolean)))

(event Ability|EventActivateAbility
  (|PlayMontageandWaitProxy "None" (select (Math|Random|RandomBool) "/Game/OpenWorldAnimset/OpenWordAnimations/Deaths/ANMTG_Death_B.ANMTG_Death_B" "/Game/OpenWorldAnimset/OpenWordAnimations/Deaths/ANMTG_Death_F.ANMTG_Death_F") 1.0 "None" true 1.0 0.0 false
    (:then
      (Utilities|FlowControl|Delay (Animation|GetPlayLength (Variables|Default|GetDeathMontage)))
      (Utilities|FlowControl|Sequence
        (:then_0
          (bind _asplayer_character_base (Utilities|Casting|CastToPlayerCharacterBase (Ability|GetOwningActorfromActorInfo)))
          (Class|SoulCharacterBase|FinishDeath _asplayer_character_base))
        (:then_1
          (Ability|EndAbility))))))