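; GA_Roll is a Gameplay Ability that makes the character perform a dodge roll via a montage.
; After committing, the locally controlled character takes yaw from its last movement input and passes it to a `Ser_`-prefixed event.
; That event sets the rotation of the "RollRotate" Motion Warping target, steering the roll toward input.
; The ability ends on montage completion or blend-out, and cancels on interruption or failed commit.
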(event Custom|Ser_UpdateWarpTargetRotation
  (params (Rot :type Rotator))
  (bind _as角色 (Utilities|Casting|CastToCharacter (Ability|GetOwningActorfromActorInfo)))
  (Utilities|IsValid (Actor|GetComponentbyClass _as角色 "/Script/MotionWarping.MotionWarpingComponent")
    (:Is%20Valid
      (Class|MotionWarpingComponent|AddorUpdateWarpTargetfromLocationandRotation (Actor|GetComponentbyClass _as角色 "/Script/MotionWarping.MotionWarpingComponent") "RollRotate" "0, 0, 0" Rot))))

(event Ability|EventActivateAbility
  (bind _returnvalue (Ability|CommitAbility))
  (if _returnvalue
    (Utilities|FlowControl|Sequence
      (:then_0
        (bind _as角色 (Utilities|Casting|CastToCharacter (Ability|GetOwningActorfromActorInfo)))
        (if (Pawn|IsLocallyControlled _as角色)
          (CallFunction|SerUpdateWarpTargetRotation (Math|Rotator|MakeRotator (.roll (Transformation|GetActorRotation _as角色)) (.pitch (Transformation|GetActorRotation _as角色)) (.yaw (Math|Conversions|RotationFromXVector (Pawn|Components|PawnMovement|GetLastInputVector (Variables|/Script/Engine.Character|GetCharacterMovement _as角色))))))))
      (:then_1
        (|PlayMontageandWaitProxy "None" "/Game/FightAnimations/ANMTG_Roll.ANMTG_Roll" 1.0 "None" true 1.0 0.0 false
          (:OnCompleted
            (Ability|EndAbility :!label _label))
          (:OnBlendOut
            (goto _label))
          (:OnInterrupted
            (Ability|CancelAbility :!label _label_2))
          (:OnCancelled
            (goto _label_2)))))
    (else
      (Ability|CancelAbility))))

(event Ability|EventOnEndAbility
  (params (bWasCancelled :type Boolean)))