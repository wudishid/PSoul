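; GA_KuLou_Nudged is an event-triggered gameplay ability that knocks the KuLou AI back when nudged.
; It applies a half-second root motion jump force using rotation and distance from the CG_HitInfo collapsed graph.
; That graph contains nodes for the instigator-to-owner direction and the impulse from the damage target data.
; The ability ends when the jump finishes or lands, keeping the last root motion velocity on finish.
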(event Ability|EventOnEndAbility
  (params (bWasCancelled :type Boolean)))

(event Ability|EventActivateAbilityFromEvent
  (params (EventData :type Gameplay%20Event%20Data%20Structure%20%28by%20ref%29))
  (bind (_rotation _distance) (|CG_HitInfo EventData))
  (|ApplyRootMotionJumpForce "None" _rotation _distance 0.0 0.5 0.0 false "MaintainLastRootMotionVelocity" "0, 0, 0" 0.0
    (:OnFinish
      _)
    (:OnLanded
      _))
  (Ability|EndAbility))