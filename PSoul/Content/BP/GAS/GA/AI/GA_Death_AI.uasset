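; GA_Death_AI is an AI gameplay ability that plays a death montage and then finalises the character's death.
; On activation it starts the montage, then waits for the montage's length plus a short fixed delay instead of relying on the montage callbacks.
; After the wait it calls FinishDeath on the owning AICharacterBase and ends the ability.
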(event Ability|EventActivateAbility
  (|PlayMontageandWaitProxy "None" (Variables|Default|GetDeathMontage) 1.0 "None" true 1.0 0.0 false
    (:then
      (Utilities|FlowControl|Delay (+ (Animation|GetPlayLength (Variables|Default|GetDeathMontage)) 2.0))
      (Utilities|FlowControl|Sequence
        (:then_0
          (bind _asaicharacter_base (Utilities|Casting|CastToAICharacterBase (Ability|GetOwningActorfromActorInfo)))
          (Class|SoulCharacterBase|FinishDeath _asaicharacter_base))
        (:then_1
          (Ability|EndAbility))))))

(event Ability|EventOnEndAbility
  (params (bWasCancelled :type Boolean)))