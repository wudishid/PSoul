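; GA_Hit is an event-triggered gameplay ability that plays a hit reaction with knockback.
; It picks a front or back montage from the event's direction and plays it while a root motion jump force moves the character.
; CG_HitInfo supplies that force, with nodes deriving rotation away from the instigator and impulse from damage target data.
; Montage completion or blend-out ends the ability, while interruption or cancellation cancels it.
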(event Ability|EventActivateAbilityFromEvent
  (params (EventData :type Gameplay%20Event%20Data%20Structure%20%28by%20ref%29))
  (bind (_rotation _distance) (|CG_HitInfo EventData))
  (|PlayMontageandWaitProxy "None" (Utilities|Select :Index (Class|SoulGameFunctionLibrary|GetEventDataDirection EventData) :Forward (Variables|Default|Get前) :Back (Variables|Default|Get后)) 1.0 "None" true 1.0 0.0 false
    (:then
      (|ApplyRootMotionJumpForce "None" _rotation _distance 0.0 0.5 0.0 false "MaintainLastRootMotionVelocity" "0, 0, 0" 0.0))
    (:OnCompleted
      (Ability|EndAbility :!label _label))
    (:OnBlendOut
      (goto _label))
    (:OnInterrupted
      (Ability|CancelAbility :!label _label_2))
    (:OnCancelled
      (goto _label_2))))

(event Ability|EventOnEndAbility
  (params (bWasCancelled :type Boolean)))