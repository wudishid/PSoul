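; Player hit-reaction gameplay ability, activated from a gameplay event, that plays a directional montage with knockback.
; A dot product between the owner's forward vector and the direction to the instigator picks the front or back montage.
; A root motion jump force pushes the owner, with rotation and distance from a collapsed hit-info graph referencing the away-from-instigator direction and damage impulse.
; The montage outcome ends or cancels the ability.
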(event Ability|EventOnEndAbility
  (params (bWasCancelled :type Boolean)))

(event Ability|EventActivateAbilityFromEvent
  (params (EventData :type Gameplay%20Event%20Data%20Structure%20%28by%20ref%29))
  (bind (_rotation _distance) (|CG_HitInfo_2 EventData))
  (Variables|Default|SetInstigatorLocation (Transformation|GetActorLocation (.Instigator (Utilities|Struct|BreakGameplayEventData EventData))))
  (Utilities|FlowControl|Sequence
    (:then_0
      (Variables|Default|SetMontage%20to%20Play (select (> (Math|Vector|DotProduct (Math|Vector|Normalize (- (Variables|Default|GetInstigatorLocation) (Transformation|GetActorLocation (Ability|GetOwningActorfromActorInfo)))) (Transformation|GetActorForwardVector (Ability|GetOwningActorfromActorInfo))) 0.0) "/Game/Animation/Common/HitReactFront_Montage.HitReactFront_Montage" "/Game/Animation/Common/HitReactBack_Montage.HitReactBack_Montage")))
    (:then_1
      (|PlayMontageandWaitProxy "None" (Variables|Default|GetMontage%20to%20Play) 1.0 "None" true 1.0 0.0 false
        (:then
          (|ApplyRootMotionJumpForce "None" _rotation _distance 0.0 0.5 0.0 false "MaintainLastRootMotionVelocity" "0, 0, 0" 0.0))
        (:OnCompleted
          (Ability|EndAbility :!label _label))
        (:OnBlendOut
          (goto _label))
        (:OnInterrupted
          (Ability|CancelAbility :!label _label_2))
        (:OnCancelled
          (goto _label_2))))))