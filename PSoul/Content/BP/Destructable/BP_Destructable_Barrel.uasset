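; Destructible barrel Blueprint that fractures when it takes damage and spawns items.
; Damage triggers Mul_Fracte, which switches the Geometry Collection's collision channel and spawns an auto-destroying FS_MasterField at the barrel to drive the break.
; Parallel delayed branches then hide the pickup effect with an explosion and sound, spawn items on authority only, and finally destroy the actor.
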(event Custom|Mul_Fracte
  (Collision|SetCollisionObjectType (Variables|Default|GetGeometryCollection) "ECC_GameTraceChannel1")
  (bind _returnvalue (Game|SpawnActorfromClass "/Engine/EditorResources/FieldNodes/FS_MasterField.FS_MasterField_C" (Transformation|GetActorTransform) "Undefined" "MultiplyWithRoot" 0 0))
  (Variables|/Engine/EditorResources/FieldNodes/FS_MasterField.FS_MasterField_C|SetActivationType _returnvalue "NewEnumerator4")
  (Variables|/Script/Engine.Actor|SetbAutoDestroyWhenFinished _returnvalue true)
  (Utilities|FlowControl|Sequence
    (:then_0
      (Utilities|FlowControl|Delay 1.0)
      (Development|SetHiddeninGame (Variables|Default|GetNS_Pickup_1) true false)
      (Effects|SpawnEmitteratLocation "/Game/InfinityBladeEffects/Effects/FX_Treasure/Resources/P_OrePile_Explosion_Basic.P_OrePile_Explosion_Basic" (Transformation|GetActorLocation))
      (Audio|PlaySoundatLocation "/Game/Free_Sounds_Pack/wav/SC_Explosion.SC_Explosion" (Transformation|GetActorLocation) "0, 0, 0" 1.0 1.0 0.0 0 0 0 0))
    (:then_1
      (Networking|SwitchHasAuthority
        (:Authority
          (Utilities|FlowControl|Delay 2.0)
          (Class|Barrel|SpawnItems))))
    (:then_2
      (Utilities|FlowControl|Delay 5.0)
      (Actor|DestroyActor))))

(event EventBeginPlay)

(event Collision|EventActorBeginOverlap
  (params (OtherActor :type Actor%20Object%20Reference)))

(event EventTick
  (params (DeltaSeconds :type Float%20%28single-precision%29)))

(event EventTakeDamage
  (CallFunction|MulFracte))

(fn ConstructionScript)