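; Modular skeleton enemy Blueprint from the UndeadPack, with configurable armor, clothing, gear and effects.
; The Construction Script binds the helmet, armor, bandage, belt, rag and quiver meshes to the main Mesh as leader pose, so they share its animation.
; Per-part boolean variables then toggle visibility of each piece, the particle effect and the bow, which also propagates to its children.
; It contains no gameplay logic, as BeginPlay is empty.
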(event EventBeginPlay)

(fn ConstructionScript
  (Components|SkinnedMesh|SetLeaderPoseComponent (Variables|Default|GetSK_HelmetPart) (Variables|Character|GetMesh) false false)
  (Utilities|FlowControl|Sequence
    (:then_0
      (Rendering|SetVisibility (Variables|Default|GetSK_Armor) (Variables|Default|GetArmorVisibility) false))
    (:then_1
      (Rendering|SetVisibility (Variables|Default|GetSK_Bandage1) (Variables|Default|GetBandage1Visibility) false))
    (:then_2
      (Rendering|SetVisibility (Variables|Default|GetSK_Bandage2) (Variables|Default|GetBandage2Visibility) false))
    (:then_3
      (Rendering|SetVisibility (Variables|Default|GetSK_Bandage3) (Variables|Default|GetBandage3Visibility) false))
    (:then_4
      (Rendering|SetVisibility (Variables|Default|GetSK_Belt) (Variables|Default|GetBeltVisibility) false))
    (:then_5
      (Rendering|SetVisibility (Variables|Default|GetSK_Helmet) (Variables|Default|GetHelmetVisibility) false))
    (:then_6
      (Rendering|SetVisibility (Variables|Default|GetSK_HelmetPart) (Variables|Default|GetHelmetPartVisibility) false))
    (:then_7
      (Rendering|SetVisibility (Variables|Default|GetSK_Quiver) (Variables|Default|GetQuiverVisibility) false))
    (:then_8
      (Rendering|SetVisibility (Variables|Default|GetSK_Rag1) (Variables|Default|GetRag1Visibility) false))
    (:then_9
      (Rendering|SetVisibility (Variables|Default|GetSK_Rag2) (Variables|Default|GetRag2Visibility) false))
    (:then_10
      (Rendering|SetVisibility (Variables|Default|GetSK_Rag3) (Variables|Default|GetRag3Visibility) false))
    (:then_11
      (Rendering|SetVisibility (Variables|Default|GetSK_Rag4) (Variables|Default|GetRag4Visibility) false))
    (:then_12
      (Rendering|SetVisibility (Variables|Default|GetSK_Rag5) (Variables|Default|GetRag5Visibility) false))
    (:then_13
      (Rendering|SetVisibility (Variables|Default|GetParticleSystem) (Variables|Default|GetFXVisibility) false))
    (:then_16
      (Rendering|SetVisibility (Variables|Default|GetSK_Bow) (Variables|Default|GetBowVisibility) true))))